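; IcePlatform is an actor, filed under Slimes, that grows wider in steps each time IncreaseScaleEvent is called.
; Each call adds IncrementalScaleConstant to the X and Y of ScaleResult, leaving Z unchanged.
; A timeline lerps from LastScale to that target while placing the actor at the supplied parent location and rotation.
; LastScale starts as the BeginPlay scale and takes the target when the timeline finishes.
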(event Custom|IncreaseScaleEvent
  (params (ParentLocation :type Vector) (ParentRotation :type Vector))
  (bind _output_get (Variables|Default|SetScaleResult (Math|Vector|MakeVector (+ (.x (Variables|Default|GetScaleResult)) (Variables|Default|GetIncrementalScaleConstant)) (+ (.y (Variables|Default|GetScaleResult)) (Variables|Default|GetIncrementalScaleConstant)) (.z (Variables|Default|GetScaleResult)))))
  (bind _newtrack_0 (Timeline|LerpInterpolationTimer PlayFromStart)
    (:Update
      (Transformation|SetActorTransform (Math|Transform|MakeTransform ParentLocation (Math|Conversions|RotationFromXVector ParentRotation) (Math|Vector|Lerp(Vector) (Variables|Default|GetLastScale) _output_get _newtrack_0))))
    (:Finished
      (Variables|Default|SetLastScale (Variables|Default|GetScaleResult)))))

(event EventBeginPlay
  (Variables|Default|SetLastScale (Class|Actor|GetActorRelativeScale3D)))

(fn ConstructionScript)