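; JumpSlime is a slime that acts as a bounce pad for the first-person character.
; Overlapping its static mesh raises the character's air control and launches it upward, scaling the character's jump velocity by a bounce multiplier.
; An IncreaseSizeEvent plays size-increase feedback, adds a fixed increment to that multiplier and prints the new value.
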(event OnComponentBeginOverlap(StaticMesh)
  (params (OverlappedComponent :type Primitive%20Component%20Object%20Reference) (OtherActor :type Actor%20Object%20Reference) (OtherComp :type Primitive%20Component%20Object%20Reference) (OtherBodyIndex :type Integer) (bFromSweep :type Boolean) (SweepResult :type Hit%20Result%20Structure%20%28by%20ref%29))
  (bind _asfirst_person_character (Utilities|Casting|CastToFirstPersonCharacter OtherActor))
  (Variables|/Script/Engine.CharacterMovementComponent|SetAirControl (Variables|/Script/Engine.Character|GetCharacterMovement _asfirst_person_character) 0.7)
  (Character|LaunchCharacter _asfirst_person_character (Math|Vector|MakeVector 0.0 0.0 (* (Variables|/Script/Engine.CharacterMovementComponent|GetJumpZVelocity (Variables|/Script/Engine.Character|GetCharacterMovement _asfirst_person_character)) (Variables|Default|GetInitialBounceMult))) false true))

(event EventBeginPlay)

(event Collision|EventActorBeginOverlap
  (params (OtherActor :type Actor%20Object%20Reference)))

(event EventTick
  (params (DeltaSeconds :type Float%20%28single-precision%29)))

(event EventIncreaseSizeEvent
  (Class|Slime|IncreaseSizeFeedback)
  (bind _output_get (Variables|Default|SetInitialBounceMult (+ (Variables|Default|GetInitialBounceMult) (Variables|Default|GetIncrementBounce))))
  (Development|PrintString (Utilities|String|ToString(Float) _output_get) true true "(R=1.000000,G=0.000000,B=0.024862,A=1.000000)"))

(fn ConstructionScript)