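; Slime actor whose weight follows its slime amount and acts on weight platforms.
; Appear and size-change events recompute the weight, with size changes also playing feedback and updating the stored platform.
; Overlapping an actor tagged WeightPlatform stores that platform and passes itself to its refresh call; nothing here clears the reference.
; Overlaps with DestructibleWall actors route to an empty handler.
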(event OnComponentBeginOverlap(CollisionMesh)
  (params (OverlappedComponent :type Primitive%20Component%20Object%20Reference) (OtherActor :type Actor%20Object%20Reference) (OtherComp :type Primitive%20Component%20Object%20Reference) (OtherBodyIndex :type Integer) (bFromSweep :type Boolean) (SweepResult :type Hit%20Result%20Structure%20%28by%20ref%29))
  ;[1 1 1] Overlap Interactions
  (if (Actor|ActorHasTag OtherActor "WeightPlatform")
    (CallFunction|InteractswithPlatform OtherActor)
    (elif (Actor|ActorHasTag OtherActor "DestructibleWall")
      (CallFunction|CollidesDestructibleWall OtherActor))))

(event EventAppearEvent
  (Class|Slime|Appear)
  (CallFunction|RefreshWeight))

(event EventTick
  (params (DeltaSeconds :type Float%20%28single-precision%29)))

(event EventIncreaseSizeEvent
  ;[1 1 1] Refresh Weight
  (Class|Slime|IncreaseSizeFeedback)
  (CallFunction|RefreshWeight)
  (CallFunction|ChangeWeightonPlatform))

(event EventDecreaseSizeEvent
  ;[1 1 1] Refresh Weight
  (Class|Slime|DecreaseSizeFeedback)
  (CallFunction|RefreshWeight)
  (CallFunction|ChangeWeightonPlatform))

(fn ConstructionScript)

(fn RefreshWeight
  (Variables|Default|SetWeight (Math|Conversions|ToFloat(Integer) (Variables|Default|GetSlimeAmount))))

(fn InteractswithPlatform
  (params (PlatformActor :type Actor%20Object%20Reference%20%28by%20ref%29))
  (bind _asbp_weight_platform (Utilities|Casting|CastTobpWeightPlatform PlatformActor))
  (Variables|Default|SetPlatform_Ref _asbp_weight_platform)
  (CallFunction|ChangeWeightonPlatform))

(fn ChangeWeightonPlatform
  (bind _platform_ref (Variables|Default|GetPlatform_Ref))
  (if (Utilities|IsValid _platform_ref)
    (Default|RefreshWeightCall _platform_ref self)))

(fn CollidesDestructibleWall
  (params (DestructibleWallActor :type Actor%20Object%20Reference%20%28by%20ref%29)))

(fn GetWeight
  (return (Variables|Default|GetWeight)))