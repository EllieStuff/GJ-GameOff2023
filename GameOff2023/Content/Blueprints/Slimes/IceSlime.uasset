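; Ice slime Blueprint that creates an ice platform when it touches water.
; The water overlap event runs the floor overlap logic, then after a short delay spawns an IcePlatform at the slime's transform and stores it.
; Size increase and decrease events scale that platform, destroying it once SlimeAmount runs out on a decrease.
; Without a valid platform, they play the size feedback instead.
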(event EventBeginPlay)

(event EventDecreaseSizeEvent
  (bind _returnvalue (Transformation|GetActorTransform))
  (bind _iceplatform_ref (Variables|Default|GetIcePlatform_Ref))
  (if (Utilities|IsValid _iceplatform_ref)
    (Default|DecreaseScaleEvent _iceplatform_ref (.location _returnvalue) (Math|Rotator|GetRotationXVector (.rotation _returnvalue)) (<= (Variables|Default|GetSlimeAmount) 0))
    (else
      (Class|Slime|DecreaseSizeFeedback))))

(event EventOnOverlapWaterEvent
  (params (OtherActor :type Actor%20Object%20Reference))
  (Class|Slime|OnOverlapFloor OtherActor)
  (Utilities|FlowControl|Delay 0.3)
  (bind _returnvalue (Game|SpawnActorfromClass "/Game/Blueprints/Slimes/IcePlatform.IcePlatform_C" (Transformation|GetActorTransform) "Undefined" 0 0))
  (Variables|Default|SetIcePlatform_Ref _returnvalue))

(event EventIncreaseSizeEvent
  (bind _returnvalue (Transformation|GetActorTransform))
  (bind _iceplatform_ref (Variables|Default|GetIcePlatform_Ref))
  (if (Utilities|IsValid _iceplatform_ref)
    (Default|IncreaseScaleEvent _iceplatform_ref (.location _returnvalue) (Math|Rotator|GetRotationXVector (.rotation _returnvalue)))
    (else
      (Class|Slime|IncreaseSizeFeedback))))

(fn ConstructionScript)

(fn NewFunction0
  (params (Actors :type Array%20of%20Actor%20Object%20References))
  (Collision|GetActorArrayBounds Actors))

(fn NewFunction1
  (params (Actors :type Array%20of%20Actor%20Object%20References))
  (Collision|GetActorArrayBounds Actors))