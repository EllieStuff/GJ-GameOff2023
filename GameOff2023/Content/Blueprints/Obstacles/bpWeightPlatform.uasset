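; Pressure platform that triggers a linked obstacle once the summed weight of registered weight slimes reaches a threshold.
; RefreshWeightCall registers a slime, then re-sums the weights, pruning invalid references and restarting the count.
; RefreshZScale fires the obstacle's enter, exit or interaction-feedback event from the result.
; A timeline lerps the mesh's Z scale down in proportion to load, clamped to a minimum, as visual compression.
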(event Custom|Lerp%20Mesh%20Scale
  (params (Target%20Mesh :type Scene%20Component%20Object%20Reference%20%28by%20ref%29) (Initial%20Size :type Vector%20%28by%20ref%29) (Target%20Size :type Vector%20%28by%20ref%29))
  (bind _lerp_time (Timeline|LerpMesh_Timeline PlayFromStart)
    (:Update
      (Transformation|SetRelativeScale3D (Variables|Default|GetStaticMesh) (Math|Vector|Lerp(Vector) Initial%20Size Target%20Size _lerp_time)))))

(event EventBeginPlay
  (Variables|Default|SetInitialZScale (.Z (Math|Vector|BreakVector (Variables|/Script/Engine.SceneComponent|GetRelativeScale3D (Variables|Default|GetStaticMesh))))))

(event Collision|EventActorBeginOverlap
  (params (OtherActor :type Actor%20Object%20Reference)))

(event EventTick
  (params (DeltaSeconds :type Float%20%28single-precision%29)))

(fn ConstructionScript)

(fn RefreshZScale
  (bind _initialzscale (Variables|Default|GetInitialZScale))
  (bind _staticmesh (Variables|Default|GetStaticMesh))
  (bind _staticmesh_2 (Variables|Default|GetStaticMesh))
  (bind _staticmesh_3 (Variables|Default|GetStaticMesh))
  (bind _relativescale3d (Variables|/Script/Engine.SceneComponent|GetRelativeScale3D _staticmesh_3))
  (bind (_x _y) (Math|Vector|BreakVector _relativescale3d))
  (if (>= (Variables|Default|GetCurrentWeight) (Variables|Default|GetWeightNeeded))
    (Default|EnterTriggerEvent (Variables|Default|GetTriggerableObstacle_Ref))
    (Variables|Default|SetObject%20Triggered true)
    (CallFunction|LerpMeshScale _staticmesh_2 (Variables|/Script/Engine.SceneComponent|GetRelativeScale3D _staticmesh_2) (Math|Vector|MakeVector _x _y (Variables|Default|GetMINIMUM_Z_SCALE)))
    (else
      (if (Variables|Default|GetObject%20Triggered)
        (Variables|Default|SetObject%20Triggered false)
        (Default|ExitTriggerEvent (Variables|Default|GetTriggerableObstacle_Ref))
        (else
          (Default|InteractionFeedbackEvent (Variables|Default|GetTriggerableObstacle_Ref))))
      (CallFunction|LerpMeshScale _staticmesh (Variables|/Script/Engine.SceneComponent|GetRelativeScale3D _staticmesh) (Math|Vector|MakeVector _x _y (Math|Float|Clamp(Float) (- _initialzscale (* (/ (Variables|Default|GetCurrentWeight) (Variables|Default|GetWeightNeeded)) _initialzscale)) (Variables|Default|GetMINIMUM_Z_SCALE) _initialzscale))))))

(fn RefreshWeightCall
  (params (WeightSlimeRef :type Bp%20Weight%20Slime%20Object%20Reference))
  (bind _weightslimesinplatform (Variables|Default|GetWeightSlimesInPlatform))
  (if (>= (Utilities|Array|FindItem _weightslimesinplatform WeightSlimeRef) 0)
    _
    (else
      (Utilities|Array|Add _weightslimesinplatform WeightSlimeRef)))
  (CallFunction|RefreshCurrentWeight))

(fn RefreshCurrentWeight
  (bind _weightslimesinplatform (Variables|Default|GetWeightSlimesInPlatform))
  (Variables|Default|SetCurrentWeight 0.0 :!label _label)
  (for _array_element _weightslimesinplatform
    (if (Utilities|IsValid _array_element)
      (bind _weight (Default|GetWeight _array_element))
      (Variables|Default|SetCurrentWeight (+ _weight (Variables|Default|GetCurrentWeight)))
      (else
        (Utilities|Array|RemoveItem _weightslimesinplatform _array_element)
        (goto _label))))
  (CallFunction|RefreshZScale))