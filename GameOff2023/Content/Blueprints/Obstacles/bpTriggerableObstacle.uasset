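; Obstacle actor with a cube that flattens when triggered and restores its height when the trigger is exited.
; On BeginPlay it caches the cube's original scale and a triggered scale with near-zero Z.
; Enter and exit trigger events each play their own timeline from the start, lerping between those scales in opposite directions.
; Restarting from the start makes an interrupted transition snap to an endpoint rather than reverse smoothly.
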(event EventBeginPlay
  (bind _cube (Variables|Default|GetCube))
  (bind _relativescale3d (Variables|/Script/Engine.SceneComponent|GetRelativeScale3D _cube))
  (bind (_x _y) (Math|Vector|BreakVector _relativescale3d))
  (|CallParentFunction)
  (Variables|Default|SetNot%20Triggered%20Scale _relativescale3d)
  (Variables|Default|SetTriggered%20Scale (Math|Vector|MakeVector _x _y 0.01)))

(event Collision|EventActorBeginOverlap
  (params (OtherActor :type Actor%20Object%20Reference))
  (|CallParentFunction OtherActor) ; This node is disabled and will not be called.\nDrag off pins to build functionality.
)

(event EventTick
  (params (DeltaSeconds :type Float%20%28single-precision%29))
  (|CallParentFunction DeltaSeconds) ; This node is disabled and will not be called.\nDrag off pins to build functionality.
)

(event EventEnterTriggerEvent
  (bind _lerp_time (Timeline|Timeline_0 PlayFromStart)
    (:Update
      (Transformation|SetRelativeScale3D (Variables|Default|GetCube) (Math|Vector|Lerp(Vector) (Variables|Default|GetNot%20Triggered%20Scale) (Variables|Default|GetTriggered%20Scale) _lerp_time)))))

(event EventExitTriggerEvent
  (bind _lerp_time (Timeline|Timeline_1 PlayFromStart)
    (:Update
      (Transformation|SetRelativeScale3D (Variables|Default|GetCube) (Math|Vector|Lerp(Vector) (Variables|Default|GetTriggered%20Scale) (Variables|Default|GetNot%20Triggered%20Scale) _lerp_time)))))

(fn ConstructionScript
  (|CallParentFunction))